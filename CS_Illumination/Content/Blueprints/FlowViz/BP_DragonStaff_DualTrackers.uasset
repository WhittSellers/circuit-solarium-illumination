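; Dual-tracker dragon staff actor that drives two quad-hub staff components from Live Link tracking data.
; Each Live Link controller's update event evaluates its named tracker subject as a Transform role.
; Valid frames set the matching hub's relative location and rotation, then apply a shared local rotation offset to calibrate mesh orientation.
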(event OnLiveLinkUpdated(LiveLinkComponentController)
  (params (DeltaTime :type Float%20%28single-precision%29))
  (bind _dragonstaff_quadhub (Variables|Default|GetDragonStaff_QuadHub))
  ;[1 1 1] Get and Apply Tracker Data
  (bind _dataresult (|EvaluateLiveLinkFramewithSpecificRole (Variables|Default|GetTracker%20Name%201) "/Script/LiveLinkInterface.LiveLinkTransformRole")
    (:then
      (Transformation|SetRelativeLocationAndRotation _dragonstaff_quadhub (.location (.transform (.FrameData (Utilities|Struct|BreakLiveLinkTransformBlueprintData _dataresult)))) (.rotation (.transform (.FrameData (Utilities|Struct|BreakLiveLinkTransformBlueprintData _dataresult)))) false false)
      (Transformation|AddLocalRotation _dragonstaff_quadhub (Variables|Default|GetMeshRotationCalibration) false false))))

(event OnLiveLinkUpdated(LiveLinkComponentController1)
  (params (DeltaTime :type Float%20%28single-precision%29))
  (bind _dragonstaff_quadhub1 (Variables|Default|GetDragonStaff_QuadHub1))
  ;[1 1 1] Get and Apply Tracker Data
  (bind _dataresult (|EvaluateLiveLinkFramewithSpecificRole (Variables|Default|GetTracker%20Name%202) "/Script/LiveLinkInterface.LiveLinkTransformRole")
    (:then
      (Transformation|SetRelativeLocationAndRotation _dragonstaff_quadhub1 (.location (.transform (.FrameData (Utilities|Struct|BreakLiveLinkTransformBlueprintData _dataresult)))) (.rotation (.transform (.FrameData (Utilities|Struct|BreakLiveLinkTransformBlueprintData _dataresult)))) false false)
      (Transformation|AddLocalRotation _dragonstaff_quadhub1 (Variables|Default|GetMeshRotationCalibration) false false))))

(fn ConstructionScript)