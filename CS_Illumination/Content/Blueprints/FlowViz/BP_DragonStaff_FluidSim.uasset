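; BP_DragonStaff_FluidSim moves two dragon staff quad hub components from live tracker data, apparently for a fluid simulation visualization.
; Two LiveLink controllers each evaluate a named tracker's transform on update and apply its location and rotation to their hub as relative values.
; An OSC receive event filters for port 7000 and reads the address path, but does nothing with the result.
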(event OnLiveLinkUpdated(LiveLinkComponentController)
  (params (DeltaTime :type Float%20%28single-precision%29))
  ;[1 1 1] Get and Apply Tracker Data
  (bind _dataresult (|EvaluateLiveLinkFramewithSpecificRole (Variables|Default|GetTracker%20Name%201) "/Script/LiveLinkInterface.LiveLinkTransformRole")
    (:then
      (Transformation|SetRelativeLocationAndRotation (Variables|Default|GetDragonStaff_QuadHub) (.location (.transform (.FrameData (Utilities|Struct|BreakLiveLinkTransformBlueprintData _dataresult)))) (.rotation (.transform (.FrameData (Utilities|Struct|BreakLiveLinkTransformBlueprintData _dataresult)))) false false))))

(event OnLiveLinkUpdated(LiveLinkComponentController1)
  (params (DeltaTime :type Float%20%28single-precision%29))
  ;[1 1 1] Get and Apply Tracker Data
  (bind _dataresult (|EvaluateLiveLinkFramewithSpecificRole (Variables|Default|GetTracker%20Name%202) "/Script/LiveLinkInterface.LiveLinkTransformRole")
    (:then
      (Transformation|SetRelativeLocationAndRotation (Variables|Default|GetDragonStaff_QuadHub1) (.location (.transform (.FrameData (Utilities|Struct|BreakLiveLinkTransformBlueprintData _dataresult)))) (.rotation (.transform (.FrameData (Utilities|Struct|BreakLiveLinkTransformBlueprintData _dataresult)))) false false))))

(event EventRecievedOSCMessage
  (params (OSC_Message :type OSC%20Message%20Structure) (Port :type Integer))
  ;[1 1 1] OSC Message In
  (switch string (Utilities|String|ToString(Integer) Port)
    (:7000
      (bind _returnvalue (Class|OSCManager|GetOSCMessageAddress OSC_Message))
      (Class|OSCManager|GetOSCAddressFullPath _returnvalue))))

(fn ConstructionScript)