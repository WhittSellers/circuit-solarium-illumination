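; Circuit Solarium LED tubes actor that sends an OSC trigger over the network when a tagged actor overlaps it.
; BeginPlay creates an OSC client with a hardcoded IP and port.
; An overlap by an actor with the collider tag builds an "/UE/EchoOverlap" message, then immediately sends TriggerVal 1 followed by 0 as a pulse.
; The K key fires the same send, bypassing the tag check.
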(event EventBeginPlay
  (bind _returnvalue (Class|OSCManager|CreateOSCClient "192.168.1.1" 10001 "" 0)))

(event Collision|EventActorBeginOverlap
  (params (OtherActor :type Actor%20Object%20Reference))
  (if (Actor|ActorHasTag OtherActor (Variables|Default|GetColliderTag))
    (bind _returnvalue (Class|OSCManager|ConvertStringtoOSCAddress "/UE/EchoOverlap"))
    (bind _returnvalue_2 (Class|OSCManager|SetOSCMessageAddress (Utilities|Struct|MakeOSCMessage) _returnvalue))
    (Utilities|FlowControl|Sequence
      (:then_0
        (bind _output_get (Variables|Default|SetTriggerVal 1))
        (bind _returnvalue_3 (Class|OSCManager|AddInt32 _returnvalue_2 _output_get))
        (Class|OSCClient|SendOSCMessage (stale EventBeginPlay _returnvalue) _returnvalue_3))
      (:then_1
        (bind _output_get_2 (Variables|Default|SetTriggerVal 0))
        (bind _returnvalue_4 (Class|OSCManager|AddInt32 _returnvalue_2 _output_get_2))
        (Class|OSCClient|SendOSCMessage (stale EventBeginPlay _returnvalue) _returnvalue_4)))))

(event EventTick
  (params (DeltaSeconds :type Float%20%28single-precision%29)))

(event Input|KeyboardEvents|K
  (params (Key :type Key%20Structure))
  (:Pressed
    (bind _returnvalue (Class|OSCManager|ConvertStringtoOSCAddress "/UE/EchoOverlap"))
    (bind _returnvalue_2 (Class|OSCManager|SetOSCMessageAddress (Utilities|Struct|MakeOSCMessage) _returnvalue))
    (Utilities|FlowControl|Sequence
      (:then_0
        (bind _output_get (Variables|Default|SetTriggerVal 1))
        (bind _returnvalue_3 (Class|OSCManager|AddInt32 _returnvalue_2 _output_get))
        (Class|OSCClient|SendOSCMessage (stale EventBeginPlay _returnvalue) _returnvalue_3))
      (:then_1
        (bind _output_get_2 (Variables|Default|SetTriggerVal 0))
        (bind _returnvalue_4 (Class|OSCManager|AddInt32 _returnvalue_2 _output_get_2))
        (Class|OSCClient|SendOSCMessage (stale EventBeginPlay _returnvalue) _returnvalue_4)))))

(fn ConstructionScript)