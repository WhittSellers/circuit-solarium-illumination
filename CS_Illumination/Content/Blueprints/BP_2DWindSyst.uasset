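; BP_2DWindSyst is a global 2D wind controller that feeds wind settings to materials and Niagara effects.
; On construction and BeginPlay, ApplyWindPreset normalizes direction and lerps between neighboring presets by a clamped intensity, though blending omits Reactivity.
; It writes direction, force and intensity into one MPC vector, and wind, turbulence, gust and push settings into an NPC.
; Individual getters and setters allow runtime overrides, with setters updating those collections directly.
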(event EventBeginPlay
  (Wind|Preset|ApplyWindPreset (Variables|Wind|GetDefaultDirection) (Variables|Wind|GetDefaultIntensity)))

(fn ConstructionScript
  (Wind|Preset|ApplyWindPreset (Variables|Wind|GetDefaultDirection) (Variables|Wind|GetDefaultIntensity)))

(fn SetWindForce
  (params (Force :type Float%20%28single-precision%29))
  (bind _direction (Variables|Wind|GetDirection))
  (bind (_x _y) (Math|Vector2D|BreakVector2D _direction))
  (bind _structout (Utilities|Struct|SetmembersinSBP_2DWindSyst_Preset (Variables|Wind|GetWind) Force))
  (bind _returnvalue (Class|NiagaraFunctionLibrary|GetNiagaraParameterCollection "/Game/Particles/Collections/NPC_2DWindSyst.NPC_2DWindSyst"))
  (Effects|Components|ParticleSystem|SetFloatParameter _returnvalue "Force" (Utilities|Struct|BreakSBP_2DWindSyst_Preset _structout))
  (Rendering|Material|SetVectorParameterValue "/Game/Materials/Collections/MPC_2DWindSyst.MPC_2DWindSyst" "WindParameters" (Utilities|Struct|MakeLinearColor _x _y (Utilities|Struct|BreakSBP_2DWindSyst_Preset (Variables|Wind|GetWind)) (Variables|Wind|Preset|GetPresetIntensity)) :!class /Script/Engine.KismetMaterialLibrary))

(fn GetWindForce
  (return (Utilities|Struct|BreakSBP_2DWindSyst_Preset (Variables|Wind|GetWind))))

(fn SetWindDirection
  (params (Direction :type Vector%202D%20Structure))
  (if (> (Math|Vector2D|DotProduct(2D) Direction Direction) 0.001)
    (Variables|Wind|SetDirection (Math|Vector2D|Normalize2D Direction))
    (else
      (bind _output_get (Variables|Wind|SetDirection "(X=1.000000,Y=0.000000)"))))
  (bind _returnvalue (Class|NiagaraFunctionLibrary|GetNiagaraParameterCollection "/Game/Particles/Collections/NPC_2DWindSyst.NPC_2DWindSyst"))
  (Class|NiagaraParameterCollectionInstance|SetVector2DParameter _returnvalue "Direction" _output_get)
  (Rendering|Material|SetVectorParameterValue "/Game/Materials/Collections/MPC_2DWindSyst.MPC_2DWindSyst" "WindParameters" (Utilities|Struct|MakeLinearColor (.X (Math|Vector2D|BreakVector2D (Variables|Wind|GetDirection))) (.Y (Math|Vector2D|BreakVector2D (Variables|Wind|GetDirection))) (Utilities|Struct|BreakSBP_2DWindSyst_Preset (Variables|Wind|GetWind)) (Variables|Wind|Preset|GetPresetIntensity)) :!class /Script/Engine.KismetMaterialLibrary))

(fn GetWindDirection
  (return (Variables|Wind|GetDirection)))

(fn SetWindTurbulenceFrequency
  (params (Frequency :type Float%20%28single-precision%29))
  (bind _structout (Utilities|Struct|SetmembersinSBP_2DWindSyst_Preset (Variables|Wind|GetWind) Frequency))
  (bind _returnvalue (Class|NiagaraFunctionLibrary|GetNiagaraParameterCollection "/Game/Particles/Collections/NPC_2DWindSyst.NPC_2DWindSyst"))
  (Effects|Components|ParticleSystem|SetFloatParameter _returnvalue "TurbulenceFrequency" (Utilities|Struct|BreakSBP_2DWindSyst_Preset _structout)))

(fn GetWindTurbulenceFrequency
  (return (Utilities|Struct|BreakSBP_2DWindSyst_Preset (Variables|Wind|GetWind))))

(fn SetWindTurbulenceStrength
  (params (Strength :type Float%20%28single-precision%29))
  (bind _structout (Utilities|Struct|SetmembersinSBP_2DWindSyst_Preset (Variables|Wind|GetWind) Strength))
  (bind _returnvalue (Class|NiagaraFunctionLibrary|GetNiagaraParameterCollection "/Game/Particles/Collections/NPC_2DWindSyst.NPC_2DWindSyst"))
  (Effects|Components|ParticleSystem|SetFloatParameter _returnvalue "TurbulenceForce" (Utilities|Struct|BreakSBP_2DWindSyst_Preset _structout)))

(fn SetWindGustStrength
  (params (Strength :type Float%20%28single-precision%29))
  (bind _structout (Utilities|Struct|SetmembersinSBP_2DWindSyst_Preset (Variables|Wind|GetWind) Strength))
  (bind _returnvalue (Class|NiagaraFunctionLibrary|GetNiagaraParameterCollection "/Game/Particles/Collections/NPC_2DWindSyst.NPC_2DWindSyst"))
  (Effects|Components|ParticleSystem|SetFloatParameter _returnvalue "Gust" (Utilities|Struct|BreakSBP_2DWindSyst_Preset _structout)))

(fn SetWindPushStrength
  (params (Strength :type Float%20%28single-precision%29))
  (bind _structout (Utilities|Struct|SetmembersinSBP_2DWindSyst_Preset (Variables|Wind|GetWind) Strength))
  (bind _returnvalue (Class|NiagaraFunctionLibrary|GetNiagaraParameterCollection "/Game/Particles/Collections/NPC_2DWindSyst.NPC_2DWindSyst"))
  (Effects|Components|ParticleSystem|SetFloatParameter _returnvalue "Push" (Utilities|Struct|BreakSBP_2DWindSyst_Preset _structout)))

(fn GetWindPushStrength
  (return (Utilities|Struct|BreakSBP_2DWindSyst_Preset (Variables|Wind|GetWind))))

(fn GetWindGustStrength
  (return (Utilities|Struct|BreakSBP_2DWindSyst_Preset (Variables|Wind|GetWind))))

(fn SetWindGustRandomizeDirection
  (params (Randomize :type Float%20%28single-precision%29))
  (bind _structout (Utilities|Struct|SetmembersinSBP_2DWindSyst_Preset (Variables|Wind|GetWind) Randomize))
  (bind _returnvalue (Class|NiagaraFunctionLibrary|GetNiagaraParameterCollection "/Game/Particles/Collections/NPC_2DWindSyst.NPC_2DWindSyst"))
  (Effects|Components|ParticleSystem|SetFloatParameter _returnvalue "RandomizeDirection" (Utilities|Struct|BreakSBP_2DWindSyst_Preset _structout)))

(fn GetWindGustRandomizeDirection
  (return (Utilities|Struct|BreakSBP_2DWindSyst_Preset (Variables|Wind|GetWind))))

(fn SetWindGustRandomizeForce
  (params (Randomize :type Float%20%28single-precision%29))
  (bind _structout (Utilities|Struct|SetmembersinSBP_2DWindSyst_Preset (Variables|Wind|GetWind) Randomize))
  (bind _returnvalue (Class|NiagaraFunctionLibrary|GetNiagaraParameterCollection "/Game/Particles/Collections/NPC_2DWindSyst.NPC_2DWindSyst"))
  (Effects|Components|ParticleSystem|SetFloatParameter _returnvalue "RandomizeForce" (Utilities|Struct|BreakSBP_2DWindSyst_Preset _structout)))

(fn GetWindGustRandomizeForce
  (return (Utilities|Struct|BreakSBP_2DWindSyst_Preset (Variables|Wind|GetWind))))

(fn SetWindGustRandomizeReactivity
  (params (Randomize :type Float%20%28single-precision%29))
  (bind _structout (Utilities|Struct|SetmembersinSBP_2DWindSyst_Preset (Variables|Wind|GetWind) Randomize))
  (bind _returnvalue (Class|NiagaraFunctionLibrary|GetNiagaraParameterCollection "/Game/Particles/Collections/NPC_2DWindSyst.NPC_2DWindSyst"))
  (Effects|Components|ParticleSystem|SetFloatParameter _returnvalue "RandomizeReactivity" (Utilities|Struct|BreakSBP_2DWindSyst_Preset _structout)))

(fn GetWindGustRandomizeReactivity
  (return (Utilities|Struct|BreakSBP_2DWindSyst_Preset (Variables|Wind|GetWind))))

(fn SetWindGustReactivity
  (params (Reactivity :type Float%20%28single-precision%29))
  (bind _structout (Utilities|Struct|SetmembersinSBP_2DWindSyst_Preset (Variables|Wind|GetWind) Reactivity))
  (bind _returnvalue (Class|NiagaraFunctionLibrary|GetNiagaraParameterCollection "/Game/Particles/Collections/NPC_2DWindSyst.NPC_2DWindSyst"))
  (Effects|Components|ParticleSystem|SetFloatParameter _returnvalue "Reactivity" (Utilities|Struct|BreakSBP_2DWindSyst_Preset _structout)))

(fn GetWindTurbulenceStrength
  (return (Utilities|Struct|BreakSBP_2DWindSyst_Preset (Variables|Wind|GetWind))))

(fn GetWindGustReactivity
  (return (Utilities|Struct|BreakSBP_2DWindSyst_Preset (Variables|Wind|GetWind))))

(fn ApplyWindPreset
  (params (Direction :type Vector%202D%20Structure) (Intensity :type Float%20%28double-precision%29))
  (bind _presets (Variables|Wind|Preset|GetPresets))
  (bind _presets_2 (Variables|Wind|Preset|GetPresets))
  (bind _presets_3 (Variables|Wind|Preset|GetPresets))
  (bind (_x _y) (Math|Vector2D|BreakVector2D (Variables|Wind|GetDirection)))
  (Wind|SetWindDirection Direction)
  (Variables|Wind|Preset|SetPresetIntensity (Math|Float|Clamp(Float) Intensity))
  (Utilities|FlowControl|Sequence
    (:then_0
      ;[1 1 1] need interpolation?
      (if (== (Variables|Wind|Preset|GetPresetIntensity) 0.0)
        (Variables|Wind|SetWind (Utilities|Array|Get(acopy) (Variables|Wind|Preset|GetPresets)))
        (elif (>= (Variables|Wind|Preset|GetPresetIntensity) 1.0)
          (Variables|Wind|SetWind (Utilities|Array|Get(acopy) _presets_2 (Utilities|Array|LastIndex _presets_2)))
          (else
            (bind _output_get (LocalVariables|SetThisPresetIntensity (* (Variables|Wind|Preset|GetPresetIntensity) (Utilities|Array|LastIndex (Variables|Wind|Preset|GetPresets)))))
            (LocalVariables|SetThisPresetIndex (Math|Float|Floor _output_get))
            (LocalVariables|SetThisPresetAlpha (Math|Float|Fraction _output_get))
            ;[1 1 1] blend preset
            (if (Utilities|Array|IsValidIndex _presets_3 (+ (LocalVariables|GetThisPresetIndex) 1))
              (Variables|Wind|SetWind (Utilities|Struct|MakeSBP_2DWindSyst_Preset (Math|Float|Lerp (.Force (Utilities|Struct|BreakSBP_2DWindSyst_Preset (Utilities|Array|Get(acopy) _presets_3 (LocalVariables|GetThisPresetIndex)))) (.Force (Utilities|Struct|BreakSBP_2DWindSyst_Preset (Utilities|Array|Get(acopy) _presets_3 (+ (LocalVariables|GetThisPresetIndex) 1)))) (LocalVariables|GetThisPresetAlpha)) 1.0 (Math|Float|Lerp (.TurbulenceFrequency (Utilities|Struct|BreakSBP_2DWindSyst_Preset (Utilities|Array|Get(acopy) _presets_3 (LocalVariables|GetThisPresetIndex)))) (.TurbulenceFrequency (Utilities|Struct|BreakSBP_2DWindSyst_Preset (Utilities|Array|Get(acopy) _presets_3 (+ (LocalVariables|GetThisPresetIndex) 1)))) (LocalVariables|GetThisPresetAlpha)) (Math|Float|Lerp (.TurbulenceStrength (Utilities|Struct|BreakSBP_2DWindSyst_Preset (Utilities|Array|Get(acopy) _presets_3 (LocalVariables|GetThisPresetIndex)))) (.TurbulenceStrength (Utilities|Struct|BreakSBP_2DWindSyst_Preset (Utilities|Array|Get(acopy) _presets_3 (+ (LocalVariables|GetThisPresetIndex) 1)))) (LocalVariables|GetThisPresetAlpha)) (Math|Float|Lerp (.GustStrength (Utilities|Struct|BreakSBP_2DWindSyst_Preset (Utilities|Array|Get(acopy) _presets_3 (LocalVariables|GetThisPresetIndex)))) (.GustStrength (Utilities|Struct|BreakSBP_2DWindSyst_Preset (Utilities|Array|Get(acopy) _presets_3 (+ (LocalVariables|GetThisPresetIndex) 1)))) (LocalVariables|GetThisPresetAlpha)) (Math|Float|Lerp (.GustRandDirection (Utilities|Struct|BreakSBP_2DWindSyst_Preset (Utilities|Array|Get(acopy) _presets_3 (LocalVariables|GetThisPresetIndex)))) (.GustRandDirection (Utilities|Struct|BreakSBP_2DWindSyst_Preset (Utilities|Array|Get(acopy) _presets_3 (+ (LocalVariables|GetThisPresetIndex) 1)))) (LocalVariables|GetThisPresetAlpha)) (Math|Float|Lerp (.GustRandForce (Utilities|Struct|BreakSBP_2DWindSyst_Preset (Utilities|Array|Get(acopy) _presets_3 (LocalVariables|GetThisPresetIndex)))) (.GustRandForce (Utilities|Struct|BreakSBP_2DWindSyst_Preset (Utilities|Array|Get(acopy) _presets_3 (+ (LocalVariables|GetThisPresetIndex) 1)))) (LocalVariables|GetThisPresetAlpha)) (Math|Float|Lerp (.GustRandReactivity (Utilities|Struct|BreakSBP_2DWindSyst_Preset (Utilities|Array|Get(acopy) _presets_3 (LocalVariables|GetThisPresetIndex)))) (.GustRandReactivity (Utilities|Struct|BreakSBP_2DWindSyst_Preset (Utilities|Array|Get(acopy) _presets_3 (+ (LocalVariables|GetThisPresetIndex) 1)))) (LocalVariables|GetThisPresetAlpha)) (Math|Float|Lerp (.PushStrength (Utilities|Struct|BreakSBP_2DWindSyst_Preset (Utilities|Array|Get(acopy) _presets_3 (LocalVariables|GetThisPresetIndex)))) (.PushStrength (Utilities|Struct|BreakSBP_2DWindSyst_Preset (Utilities|Array|Get(acopy) _presets_3 (+ (LocalVariables|GetThisPresetIndex) 1)))) (LocalVariables|GetThisPresetAlpha))))
              (else
                (Variables|Wind|SetWind (Utilities|Array|Get(acopy) _presets (Utilities|Array|LastIndex _presets))) ; safety precaution
              ))))))
    (:then_1
      ;[1 1 1] apply settings to MPC
      (Rendering|Material|SetVectorParameterValue "/Game/Materials/Collections/MPC_2DWindSyst.MPC_2DWindSyst" "WindParameters" (Utilities|Struct|MakeLinearColor _x _y (Utilities|Struct|BreakSBP_2DWindSyst_Preset (Variables|Wind|GetWind)) (Variables|Wind|Preset|GetPresetIntensity)) :!class /Script/Engine.KismetMaterialLibrary))
    (:then_2
      ;[1 1 1] apply settings to NPC
      (bind _returnvalue (Class|NiagaraFunctionLibrary|GetNiagaraParameterCollection "/Game/Particles/Collections/NPC_2DWindSyst.NPC_2DWindSyst"))
      (Effects|Components|ParticleSystem|SetFloatParameter _returnvalue "Force" (.Force (Utilities|Struct|BreakSBP_2DWindSyst_Preset (Variables|Wind|GetWind))))
      (Effects|Components|ParticleSystem|SetFloatParameter _returnvalue "Reactivity" (.Reactivity (Utilities|Struct|BreakSBP_2DWindSyst_Preset (Variables|Wind|GetWind))))
      (Effects|Components|ParticleSystem|SetFloatParameter _returnvalue "TurbulenceFrequency" (.TurbulenceFrequency (Utilities|Struct|BreakSBP_2DWindSyst_Preset (Variables|Wind|GetWind))))
      (Effects|Components|ParticleSystem|SetFloatParameter _returnvalue "TurbulenceForce" (.TurbulenceStrength (Utilities|Struct|BreakSBP_2DWindSyst_Preset (Variables|Wind|GetWind))))
      (Effects|Components|ParticleSystem|SetFloatParameter _returnvalue "Gust" (.GustStrength (Utilities|Struct|BreakSBP_2DWindSyst_Preset (Variables|Wind|GetWind))))
      (Effects|Components|ParticleSystem|SetFloatParameter _returnvalue "RandomizeDirection" (.GustRandDirection (Utilities|Struct|BreakSBP_2DWindSyst_Preset (Variables|Wind|GetWind))))
      (Effects|Components|ParticleSystem|SetFloatParameter _returnvalue "RandomizeForce" (.GustRandForce (Utilities|Struct|BreakSBP_2DWindSyst_Preset (Variables|Wind|GetWind))))
      (Effects|Components|ParticleSystem|SetFloatParameter _returnvalue "RandomizeReactivity" (.GustRandReactivity (Utilities|Struct|BreakSBP_2DWindSyst_Preset (Variables|Wind|GetWind))))
      (Effects|Components|ParticleSystem|SetFloatParameter _returnvalue "Push" (.PushStrength (Utilities|Struct|BreakSBP_2DWindSyst_Preset (Variables|Wind|GetWind)))))))

(fn GetWindPresetIntensity
  (return (Variables|Wind|Preset|GetPresetIntensity)))