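; BP_TouchOSCLink is an actor that receives TouchOSC messages to remote-control level streaming, sun rotation and wind.
; On BeginPlay it starts a listening OSC server and finds the BP_LevelStreamer in the world.
; A switch on each message's address path forwards toggles to the streamer, maps two faders to sun pitch and yaw, and passes a third to UpdateWindSystem.
; Address routing is hardcoded, marked for rework once custom TouchOSC messages exist.
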(event Custom|OnMessageRecieved
  (params (Message :type OSC%20Message%20Structure%20%28by%20ref%29) (IPAddress :type String) (Port :type Integer))
  (bind _output_get (Variables|Default|SetMessage Message))
  (bind _returnvalue (Class|OSCManager|GetOSCMessageAddress _output_get))
  (bind _returnvalue_2 (Class|OSCManager|GetOSCAddressFullPath _returnvalue))
  ;[1 1 1] Select Which Manager to send message to based on string(this will need to be reworked once custom touchOSC messages are implemented)
  (switch string _returnvalue_2
    (:/1/toggle1
      (Class|BPIMessageRouting|UpdateStreamingLevels(Message) (Variables|Default|GetLevelStreamer) _output_get :!label _label)
      ;[1 1 1] Print Debug Messages
      (if (Variables|Default|GetPrintDebug)
        (bind _value (Class|OSCManager|GetFloat _output_get))
        (Development|PrintString (Utilities|String|Append _returnvalue_2 "/ " (Utilities|String|ToString(Float) _value)))
        (Class|OSCManager|ClearMessage (Variables|Default|GetMessage) :!label _label_2)))
    (:/1/toggle2
      (goto _label))
    (:/1/toggle3
      (goto _label))
    (:/1/toggle4
      (goto _label))
    (:/1/fader1
      ;[1 1 1] Sun Controls
      (bind _value_2 (Class|OSCManager|GetFloat _output_get))
      (Transformation|SetActorRotation (Variables|Default|Getsun) (Math|Rotator|MakeRotator 0.0 (Math|Float|MapRangeClamped _value_2 0.0 1.0 1.8e+02 3.6e+02) (Math|Float|MapRangeClamped (stale _value_3) 0.0 1.0 0.0 3.6e+02)))
      (goto _label_2))
    (:/1/fader2
      (bind _value_3 (Class|OSCManager|GetFloat _output_get))
      (Transformation|SetActorRotation (Variables|Default|Getsun) (Math|Rotator|MakeRotator 0.0 (Math|Float|MapRangeClamped _value_2 0.0 1.0 1.8e+02 3.6e+02) (Math|Float|MapRangeClamped _value_3 0.0 1.0 0.0 3.6e+02)))
      (goto _label_2))
    (:/1/fader3
      (CallFunction|UpdateWindSystem _output_get)
      (goto _label_2))))

(event EventBeginPlay
  (bind _returnvalue (Class|OSCManager|CreateOSCServer (Variables|Default|GetHost%20IPAddress) (Variables|Default|GetPort) false true "TouchOSC" 0))
  (bind _output_get (Variables|Default|SetTouchOSCServer _returnvalue))
  (EventDispatchers|BindEventtoOnOscMessageReceived _output_get (delegate Custom|OnMessageRecieved))
  (bind _returnvalue_2 (Actor|GetActorOfClass (Variables|Default|GetLevelStreamerActor%20Class)))
  (bind _asbp_level_streamer (Utilities|Casting|CastToBP_LevelStreamer _returnvalue_2))
  (Variables|Default|SetLevelStreamer _asbp_level_streamer))

(event Collision|EventActorBeginOverlap
  (params (OtherActor :type Actor%20Object%20Reference)))

(event EventTick
  (params (DeltaSeconds :type Float%20%28single-precision%29)))

(fn ConstructionScript)

(fn UpdateStreamingLevels
  (params (OSC_Message :type OSC%20Message%20Structure))
  (return))