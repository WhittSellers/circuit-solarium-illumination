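; BP_LevelStreamer loads and unloads four streamed levels in response to OSC messages.
; UpdateStreamingLevels switches on the message's address path, one toggle address per level, and treats a first float of 1.0 as load and any other value as unload.
; Loads become visible on completion, and neither operation blocks.
; Toggles 2 through 4 share the MatrixLevelActive flag, while toggle 1 uses GrassLevelActive.
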(event EventBeginPlay)

(event Collision|EventActorBeginOverlap
  (params (OtherActor :type Actor%20Object%20Reference)))

(event EventTick
  (params (DeltaSeconds :type Float%20%28single-precision%29)))

(event EventUpdateStreamingLevels
  (params (OSC_Message :type OSC%20Message%20Structure))
  (bind _level1 (Variables|Default|GetLevel1))
  (bind _level4 (Variables|Default|GetLevel4))
  (bind _level2 (Variables|Default|GetLevel2))
  (bind _level3 (Variables|Default|GetLevel3))
  (bind _output_get (Variables|Default|SetOSC%20Message OSC_Message))
  (bind _returnvalue (Class|OSCManager|GetOSCMessageAddress _output_get))
  (bind _returnvalue_2 (Class|OSCManager|GetOSCAddressFullPath _returnvalue))
  (switch string _returnvalue_2
    (:/1/toggle1
      (bind _value (Class|OSCManager|GetFloat (Variables|Default|GetOSC%20Message)))
      (Variables|Default|SetGrassLevelActive (== _value 1.0))
      (if (Variables|Default|GetGrassLevelActive)
        (Game|LoadStreamLevel(byName) _level1 true)
        (else
          (Game|UnloadStreamLevel(byName) _level1 false))))
    (:/1/toggle2
      (bind _value_2 (Class|OSCManager|GetFloat (Variables|Default|GetOSC%20Message)))
      (Variables|Default|SetMatrixLevelActive (== _value_2 1.0))
      (if (Variables|Default|GetMatrixLevelActive)
        (Game|LoadStreamLevel(byName) _level2 true)
        (else
          (Game|UnloadStreamLevel(byName) _level2 false))))
    (:/1/toggle3
      (bind _value_3 (Class|OSCManager|GetFloat (Variables|Default|GetOSC%20Message)))
      (Variables|Default|SetMatrixLevelActive (== _value_3 1.0))
      (if (Variables|Default|GetMatrixLevelActive)
        (Game|LoadStreamLevel(byName) _level3 true)
        (else
          (Game|UnloadStreamLevel(byName) _level3 false))))
    (:/1/toggle4
      (bind _value_4 (Class|OSCManager|GetFloat (Variables|Default|GetOSC%20Message)))
      (Variables|Default|SetMatrixLevelActive (== _value_4 1.0))
      (if (Variables|Default|GetMatrixLevelActive)
        (Game|LoadStreamLevel(byName) _level4 true)
        (else
          (Game|UnloadStreamLevel(byName) _level4 false))))))

(fn ConstructionScript)